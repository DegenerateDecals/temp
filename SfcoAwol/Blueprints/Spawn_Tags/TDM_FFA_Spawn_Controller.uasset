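; Spawn controller actor that swaps player spawn points for free-for-all or team deathmatch matches.
; On BeginPlay it reads the free-for-all flag from the Zomboy game mode, waits briefly, then destroys all existing CS_DynamicPlayerStart actors.
; It collects the transforms of the SfcoAwol FFA or TDM spawn marker actors, depending on the mode, and spawns a new CS_DynamicPlayerStart at each one.
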(event `self.ReceiveBeginPlay`
  (bind _returnvalue (`ZomboyGameMode.IsFreeForAll` (`ZomboyBlueprintLibrary.GetZomboyGameMode`)))
  (`KismetSystemLibrary.Delay` 2.0)
  ;[1 1 1] Delete cs_dynamic_PlayerStart
  (bind _outactors (`GameplayStatics.GetAllActorsOfClass` "/Game/MapUtilities/PlayerStart/CS_DynamicPlayerStart.CS_DynamicPlayerStart_C"))
  (for _array_element _outactors
    (`self.K2_DestroyActor` _array_element))
  ;[1 1 1] get custom spawn locations
  (if _returnvalue
    (bind _outactors_2 (`GameplayStatics.GetAllActorsOfClass` "/Game/SfcoAwol/Blueprint/Spawn_Tags/SfcoAwol_FAA_Spawn.SfcoAwol_FAA_Spawn_C"))
    (for _array_element_2 _outactors_2
      (`KismetArrayLibrary.Array_Add` (`self.FFA Spawners`) (`self.GetTransform` _array_element_2)))
    ;[1 1 1] FFA TDM Spawn Filter
    (for _array_element_3 (`self.FFA Spawners`)
      (`|SpawnActorFromClass` "/Game/MapUtilities/PlayerStart/CS_DynamicPlayerStart.CS_DynamicPlayerStart_C" _array_element_3 "Undefined" "OverrideRootScale" null null))
    (else
      (bind _outactors_3 (`GameplayStatics.GetAllActorsOfClass` "/Game/SfcoAwol/Blueprint/Spawn_Tags/SfcoAwol_TDM_Spawn.SfcoAwol_TDM_Spawn_C"))
      (for _array_element_4 _outactors_3
        (`KismetArrayLibrary.Array_Add` (`self.TDM Spawners`) (`self.GetTransform` _array_element_4)))
      (for _array_element_5 (`self.TDM Spawners`)
        (`|SpawnActorFromClass` "/Game/MapUtilities/PlayerStart/CS_DynamicPlayerStart.CS_DynamicPlayerStart_C" _array_element_5 "Undefined" "OverrideRootScale" null null)))))

(fn `UserConstructionScript`)